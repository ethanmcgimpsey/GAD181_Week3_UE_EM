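; BP_Key is a collectible key pickup that the player gains by entering its collection area.
; On overlap it checks the IsPlayerCarryingTheKey flag on a referenced KeyManager, so only one key can be carried at a time.
; If the flag is clear, it sets it and destroys itself; otherwise the key stays, with debug prints reporting each outcome.
; The overlap handler does not filter which actor entered.
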(event `self.Key Collection Area.OnComponentBeginOverlap`
  (params (OverlappedComponent :type "PrimitiveComponent Object Reference") (OtherActor :type "Actor Object Reference") (OtherComp :type "PrimitiveComponent Object Reference") (OtherBodyIndex :type Integer) (bFromSweep :type Boolean) (SweepResult :type "HitResult Structure (by ref)"))
  (`KismetSystemLibrary.PrintString` "Player has entered the KEY area")
  (if (`/Game/Blueprints/BP_KeyManager.isPlayerCarryingTheKey` (`self.KeyManager`))
    (`KismetSystemLibrary.PrintString` "No key collected. Player is already carrying a key.")
    (else
      (set `/Game/Blueprints/BP_KeyManager.isPlayerCarryingTheKey` true (`self.KeyManager`))
      (`KismetSystemLibrary.PrintString` (`KismetStringLibrary.Conv_BoolToString` (`/Game/Blueprints/BP_KeyManager.isPlayerCarryingTheKey` (`self.KeyManager`))))
      (`self.K2_DestroyActor`))))

(fn `UserConstructionScript`)